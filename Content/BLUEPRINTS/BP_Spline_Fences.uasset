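; Spline-driven fence Blueprint that lays a deformed mesh along an editable spline.
; The construction script adds one spline mesh component per segment, with configurable mesh, material and forward axis, bent using the local locations and tangents of adjacent points.
; Each segment gets query-only collision, and the Spline is attached to each new segment rather than the reverse.
; The event graph holds no active logic.
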(fn `UserConstructionScript`
  ; Spawns mesh instances along the spline
  (for _index (range (+ (- (`SplineComponent.GetNumberOfSplinePoints` (`self.Spline`)) 2) 1))
    (bind _returnvalue (`AddComponent|NODE_AddSplineMeshComponent-0`))
    (`/Engine/EditorBlueprintResources/StandardMacros.IsValid` _returnvalue
      (:`Is Valid`
        (`StaticMeshComponent.SetStaticMesh` _returnvalue (`self.Mesh`))
        (`PrimitiveComponent.SetMaterial` _returnvalue 0 (`self.Material`))
        (`SplineMeshComponent.SetForwardAxis` _returnvalue (`self.Axis`) true)
        (`SceneComponent.K2_AttachToComponent` (`self.Spline`) _returnvalue "None" "KeepRelative" "KeepRelative" "KeepRelative" true)
        (bind (_location _tangent) (`SplineComponent.GetLocationAndTangentAtSplinePoint` (`self.Spline`) _index "Local"))
        (bind (_location_2 _tangent_2) (`SplineComponent.GetLocationAndTangentAtSplinePoint` (`self.Spline`) (+ _index 1) "Local"))
        (`SplineMeshComponent.SetStartAndEnd` _returnvalue _location _tangent _location_2 _tangent_2 true)
        (`PrimitiveComponent.SetCollisionEnabled` _returnvalue "QueryOnly")))))