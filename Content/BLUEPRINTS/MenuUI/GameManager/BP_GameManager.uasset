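; BP_GameManager handles level progress and audio settings persistence for the game.
; Level and settings use separate save slots of BP_SaveCurrentState, with the saved level name reopened on load.
; Music and SFX volumes apply immediately through MasterMix sound class overrides, are written by SaveSettings, and are restored by LoadSettings.
; A lowercase level-name substring check blocks saving and pausing on excluded levels.
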(event `Save Level`
  ;[1 1 1] Level loading and saving
  (`|ExecutionSequence`
    (:`then_0`
      (`/Engine/EditorBlueprintResources/StandardMacros.DoOnce` false
        (:`Completed`
          (bind _returnvalue (`GameplayStatics.CreateSaveGameObject` "/Game/BLUEPRINTS/MenuUI/GameManager/BP_SaveCurrentState.BP_SaveCurrentState_C"))
          (bind _output_get (set `self.SaveGameObject` _returnvalue)))))
    (:`then_1`
      (bind _returnvalue_2 (`GameplayStatics.GetCurrentLevelName` true))
      (bind _cansave (`self.CanSaveLevel` _returnvalue_2))
      (if _cansave
        (set `/Game/BLUEPRINTS/MenuUI/GameManager/BP_SaveCurrentState.CurrentLevel` (`KismetStringLibrary.Conv_StringToName` _returnvalue_2) _output_get)
        (`GameplayStatics.SaveGameToSlot` _output_get (`self.SlotName`))))))

(event `Load Level`
  ;[1 1 1] Level loading and saving
  (bind _returnvalue (`GameplayStatics.LoadGameFromSlot` (`self.SlotName`)))
  (bind _asbp_save_current_state (cast `/Game/BLUEPRINTS/MenuUI/GameManager/BP_SaveCurrentState` _returnvalue))
  (`GameplayStatics.OpenLevel` (`/Game/BLUEPRINTS/MenuUI/GameManager/BP_SaveCurrentState.CurrentLevel` _asbp_save_current_state)))

(event `SaveSetting`
  (params (Value :type "Float (double-precision)") (Setting :type "/Game/BLUEPRINTS/MenuUI/GameManager/ESettings Enum" :default "NewEnumerator0"))
  ;[1 1 1] Settings
  (switch `/Game/BLUEPRINTS/MenuUI/GameManager/ESettings` Setting
    (:`NewEnumerator0`
      (bind _output_get (set `self.MusicVolumeSaved` Value))
      (`GameplayStatics.SetSoundMixClassOverride` "/Game/BLUEPRINTS/MenuUI/GameManager/SoundClasses/MasterMix.MasterMix" "/Game/BLUEPRINTS/MenuUI/GameManager/SoundClasses/Music.Music" _output_get))
    (:`NewEnumerator1`
      (bind _output_get_2 (set `self.SFXVolumeSaved` Value))
      (`GameplayStatics.SetSoundMixClassOverride` "/Game/BLUEPRINTS/MenuUI/GameManager/SoundClasses/MasterMix.MasterMix" "/Game/BLUEPRINTS/MenuUI/GameManager/SoundClasses/SFX.SFX" _output_get_2))))

(event `SaveSettings`
  ;[1 1 1] Settings
  (`|ExecutionSequence`
    (:`then_0`
      (`/Engine/EditorBlueprintResources/StandardMacros.DoOnce` false
        (:`Completed`
          (bind _returnvalue (`GameplayStatics.CreateSaveGameObject` "/Game/BLUEPRINTS/MenuUI/GameManager/BP_SaveCurrentState.BP_SaveCurrentState_C"))
          (bind _output_get (set `self.SaveGameObject` _returnvalue)))))
    (:`then_1`
      (set `/Game/BLUEPRINTS/MenuUI/GameManager/BP_SaveCurrentState.MusicVolume` (`self.MusicVolumeSaved`) _output_get)
      (set `/Game/BLUEPRINTS/MenuUI/GameManager/BP_SaveCurrentState.SFXVolume` (`self.SFXVolumeSaved`) _output_get)
      (`GameplayStatics.SaveGameToSlot` _output_get (`self.SlotName_Settings`)))))

(event `Load Settings`
  ;[1 1 1] Settings
  (`GameplayStatics.PushSoundMixModifier` "/Game/BLUEPRINTS/MenuUI/GameManager/SoundClasses/MasterMix.MasterMix")
  (`self.RestoreSettings`))

(fn `CanPauseLevel`
  (returns (CanPause :type Boolean))
  (bind _returnvalue (`GameplayStatics.GetCurrentLevelName` true))
  (return (not (`KismetStringLibrary.Contains` (`KismetStringLibrary.ToLower` _returnvalue) (`self.ExcludedLevelsString`)))) ; If it contains the word "map" it cannot save
)

(fn `CanSaveLevel`
  (params (LevelName :type String))
  (returns (CanSave :type Boolean))
  (return (not (`KismetStringLibrary.Contains` (`KismetStringLibrary.ToLower` LevelName) (`self.ExcludedLevelsString`)))) ; If it contains the word "map" it cannot save
)

(fn `HasSavedLevel`
  (returns (HasSavedLevel :type Boolean))
  (bind _returnvalue (`GameplayStatics.LoadGameFromSlot` (`self.SlotName`)))
  (bind _asbp_save_current_state (cast `/Game/BLUEPRINTS/MenuUI/GameManager/BP_SaveCurrentState` _returnvalue))
  (return (not (== (`/Game/BLUEPRINTS/MenuUI/GameManager/BP_SaveCurrentState.CurrentLevel` _asbp_save_current_state) "None"))))

(fn `RestoreSettings`
  (bind _returnvalue (`GameplayStatics.LoadGameFromSlot` (`self.SlotName_Settings`)))
  (bind _asbp_save_current_state (cast `/Game/BLUEPRINTS/MenuUI/GameManager/BP_SaveCurrentState` _returnvalue))
  (bind _output_get (set `self.MusicVolumeSaved` (`/Game/BLUEPRINTS/MenuUI/GameManager/BP_SaveCurrentState.MusicVolume` _asbp_save_current_state)))
  (`GameplayStatics.SetSoundMixClassOverride` "/Game/BLUEPRINTS/MenuUI/GameManager/SoundClasses/MasterMix.MasterMix" "/Game/BLUEPRINTS/MenuUI/GameManager/SoundClasses/Music.Music" _output_get)
  (bind _output_get_2 (set `self.SFXVolumeSaved` (`/Game/BLUEPRINTS/MenuUI/GameManager/BP_SaveCurrentState.SFXVolume` _asbp_save_current_state)))
  (`GameplayStatics.SetSoundMixClassOverride` "/Game/BLUEPRINTS/MenuUI/GameManager/SoundClasses/MasterMix.MasterMix" "/Game/BLUEPRINTS/MenuUI/GameManager/SoundClasses/SFX.SFX" _output_get_2))