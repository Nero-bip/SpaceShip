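; BP_RotateObjects is an inspectable world item with a configurable mesh, material, description and two-stage proximity prompts.
; The construction script applies the model and sphere radii, and player overlaps with the outer and inner spheres switch between the two interaction indicators.
; InspectItem hides the item with a sound and triggers BPCObjetos text, while InspectComplete restores it and removes the text; both return the item's data.
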(event `self.ReceiveBeginPlay`
  (`PrimitiveComponent.SetMaterial` (`self.StaticMesh`) 0 (`self.Material`)))

(event `DestroyItem`
  (`GameplayStatics.PlaySound2D` (`self.Sound`) 1.0 1.0 0.0 null null)
  (`/Game/FirstPerson/Dialogue/BPC_Objetos.Texto` (`self.BPC_Objetos`))
  (`KismetSystemLibrary.Delay` 0.02)
  (`SceneComponent.SetVisibility` (`self.StaticMesh`) false false)
  (`PrimitiveComponent.SetMaterial` (`self.MaterialBillboard`) 0 null)
  (`SceneComponent.SetVisibility` (`self.InnerInteraction`) false false)
  (`SceneComponent.SetVisibility` (`self.OuterInteraction`) false false))

(event `ItemVisible`
  (`/Game/FirstPerson/Dialogue/BPC_Objetos.Remove_Text` (`self.BPC_Objetos`))
  (`KismetSystemLibrary.Delay` 0.0)
  (`SceneComponent.SetVisibility` (`self.StaticMesh`) true false)
  (`PrimitiveComponent.SetMaterial` (`self.MaterialBillboard`) 0 null)
  (`SceneComponent.SetVisibility` (`self.InnerInteraction`) true false)
  (`SceneComponent.SetVisibility` (`self.OuterInteraction`) false false))

(event `self.OuterSphereCollision.OnComponentBeginOverlap`
  (params (OverlappedComponent :type "PrimitiveComponent Object Reference") (OtherActor :type "Actor Object Reference") (OtherComp :type "PrimitiveComponent Object Reference") (OtherBodyIndex :type Integer) (bFromSweep :type Boolean) (SweepResult :type "HitResult Structure (by ref)"))
  (if (== OtherActor (`GameplayStatics.GetPlayerCharacter` 0))
    (`SceneComponent.SetVisibility` (`self.OuterInteraction`) true false)))

(event `self.OuterSphereCollision.OnComponentEndOverlap`
  (params (OverlappedComponent :type "PrimitiveComponent Object Reference") (OtherActor :type "Actor Object Reference") (OtherComp :type "PrimitiveComponent Object Reference") (OtherBodyIndex :type Integer))
  (if (== (`GameplayStatics.GetPlayerCharacter` 0) OtherActor)
    (`SceneComponent.SetVisibility` (`self.OuterInteraction`) false false)))

(event `self.InnerSphereCollision.OnComponentBeginOverlap`
  (params (OverlappedComponent :type "PrimitiveComponent Object Reference") (OtherActor :type "Actor Object Reference") (OtherComp :type "PrimitiveComponent Object Reference") (OtherBodyIndex :type Integer) (bFromSweep :type Boolean) (SweepResult :type "HitResult Structure (by ref)"))
  (if (== OtherActor (`GameplayStatics.GetPlayerCharacter` 0))
    (`SceneComponent.SetVisibility` (`self.InnerInteraction`) true false)
    (`SceneComponent.SetVisibility` (`self.OuterInteraction`) false false)))

(event `self.InnerSphereCollision.OnComponentEndOverlap`
  (params (OverlappedComponent :type "PrimitiveComponent Object Reference") (OtherActor :type "Actor Object Reference") (OtherComp :type "PrimitiveComponent Object Reference") (OtherBodyIndex :type Integer))
  (if (== (`GameplayStatics.GetPlayerCharacter` 0) OtherActor)
    (`SceneComponent.SetVisibility` (`self.InnerInteraction`) false false)
    (`SceneComponent.SetVisibility` (`self.OuterInteraction`) true false)))

(fn `InspectComplete`
  (returns (ItemModel :type "StaticMesh Object Reference") (Material :type "MaterialInterface Object Reference") (ItemDescript :type Text))
  (`self.ItemVisible`)
  (return (`self.ItemModel`) (`self.Material`) (`self.ItemDescription`)))

(fn `InspectItem`
  (returns (`Item Model` :type "StaticMesh Object Reference") (Material :type "MaterialInterface Object Reference") (`Item Description` :type Text))
  (`self.DestroyItem`)
  (return (`self.ItemModel`) (`self.Material`) (`self.ItemDescription`)))

(fn `UserConstructionScript`
  (`StaticMeshComponent.SetStaticMesh` (`self.StaticMesh`) (`self.ItemModel`))
  (`PrimitiveComponent.SetMaterial` (`self.StaticMesh`) 0 (`self.Material`))
  (`SphereComponent.SetSphereRadius` (`self.InnerSphereCollision`) (`self.InnerSphereRadius`) true)
  (`SphereComponent.SetSphereRadius` (`self.OuterSphereCollision`) (`self.OuterSphereRadius`) true))